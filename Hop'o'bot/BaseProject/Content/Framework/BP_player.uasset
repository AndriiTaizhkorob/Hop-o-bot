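; First-person player character Blueprint that handles movement, climbing, interaction, pausing and HUD setup.
; On BeginPlay it adds the Enhanced Input mapping context and HUD; input events drive look, jump, movement and a game-pausing menu.
; While IsClimbing is true, movement switches to Flying mode and forward input moves along the up vector.
; Interact and PlaceItem delegate to the CPPInventory component, and overlapping a BP_Collectable plays an orb sound.
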(event `self.ReceiveBeginPlay`
  (bind _asplayer_controller (cast `PlayerController` (`self.GetController`)))
  (bind _returnvalue (pcsubsystem `EnhancedInputLocalPlayerSubsystem` _asplayer_controller))
  (`/Engine/EditorBlueprintResources/StandardMacros.IsValid` _returnvalue
    (:`Is Valid`
      (`EnhancedInputSubsystemInterface.AddMappingContext` _returnvalue "/Game/Input/FPS_IMC.FPS_IMC" 0 (struct))
      (bind _returnvalue_2 (`|CreateWidget` "/Game/UI/WB_HUD.WB_HUD_C"))
      (bind _output_get (set `self.WB_Hud_ref` _returnvalue_2))
      (`UserWidget.AddToViewport` _output_get 0))))

(event `EnhancedInput|/Game/Input/Movement_IA`
  (params (ActionValue :type "Vector2D Structure") (ElapsedSeconds :type "Float (double-precision)") (TriggeredSeconds :type "Float (double-precision)") (InputAction :type "InputAction Object Reference" :default "/Game/Input/Movement_IA.Movement_IA"))
  (:`Triggered`
    (if (`self.IsClimbing`)
      (`self.AddMovementInput` (0.0 0.0 0.0))
      (`CharacterMovementComponent.SetMovementMode` (`self.CharacterMovement`) "MOVE_Flying" 0)
      (`self.AddMovementInput` (`self.GetActorUpVector` (`GameplayStatics.GetPlayerCharacter` 0)) ActionValue_Y)
      (else
        (`self.AddMovementInput` (`self.GetActorRightVector`) ActionValue_X)
        (`self.AddMovementInput` (`self.GetActorForwardVector`) ActionValue_Y)))))

(event `EnhancedInput|/Game/Input/Look_IA`
  (params (ActionValue :type "Vector2D Structure") (ElapsedSeconds :type "Float (double-precision)") (TriggeredSeconds :type "Float (double-precision)") (InputAction :type "InputAction Object Reference" :default "/Game/Input/Look_IA.Look_IA"))
  (:`Triggered`
    (`self.AddControllerYawInput` ActionValue_X)
    (`self.AddControllerPitchInput` ActionValue_Y)))

(event `EnhancedInput|/Game/Input/Jump_IA`
  (params (ActionValue :type Boolean) (ElapsedSeconds :type "Float (double-precision)") (TriggeredSeconds :type "Float (double-precision)") (InputAction :type "InputAction Object Reference" :default "/Game/Input/Jump_IA.Jump_IA"))
  (:`Started`
    (`self.Jump`))
  (:`Completed`
    (`self.StopJumping`)))

(event `EnhancedInput|/Game/Input/Pause_IA`
  (params (ActionValue :type Boolean) (ElapsedSeconds :type "Float (double-precision)") (TriggeredSeconds :type "Float (double-precision)") (InputAction :type "InputAction Object Reference" :default "/Game/Input/Pause_IA.Pause_IA"))
  (:`Triggered`
    (bind _returnvalue (`|CreateWidget` "/Game/UI/WB_PauseMenu.WB_PauseMenu_C"))
    (set `PlayerController.bShowMouseCursor` true (`GameplayStatics.GetPlayerController` 0))
    (`UserWidget.AddToViewport` _returnvalue 0)
    (`GameplayStatics.SetGamePaused` true)))

(event `self.CapsuleComponent.OnComponentBeginOverlap`
  (params (OverlappedComponent :type "PrimitiveComponent Object Reference") (OtherActor :type "Actor Object Reference") (OtherComp :type "PrimitiveComponent Object Reference") (OtherBodyIndex :type Integer) (bFromSweep :type Boolean) (SweepResult :type "HitResult Structure (by ref)"))
  (cast `/Game/Objects/Interactable/BP_Collectable` OtherActor)
  (`AudioComponent.Play` (`self.SFX_Orb`) 0.0))

(event `InputAction|Interact`
  (params (Key :type "Key Structure"))
  (:`Pressed`
    (`CPP_InventoryComponent.TryInteract` (`self.CPP_Inventory`) (`self.Camera`))))

(event `InputAction|PlaceItem`
  (params (Key :type "Key Structure"))
  (:`Pressed`
    (`CPP_InventoryComponent.PlaceItem` (`self.CPP_Inventory`) (+ (`self.K2_GetActorLocation`) (* (`self.GetActorForwardVector`) (`self.Multiplier`))))))

(fn `UserConstructionScript`)