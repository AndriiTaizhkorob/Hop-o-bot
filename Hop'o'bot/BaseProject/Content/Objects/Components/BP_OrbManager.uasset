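; BP_OrbManager is a component that tracks the orb count and shows it on the HUD.
; AddOrbs adds the given amount to Orbs, then calls UpdateOrbs.
; UpdateOrbs casts player character 0 to BP_player and passes the count as text to its HUD widget through UIUpdate.
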(fn `AddOrbs`
  (params (AddOrbs :type Integer))
  (set `self.Orbs` (+ AddOrbs (`self.Orbs`)))
  (`self.UpdateOrbs`))

(fn `UpdateOrbs`
  (bind _asbp_player (cast `/Game/Framework/BP_player` (`GameplayStatics.GetPlayerCharacter` 0)))
  (`/Game/UI/WB_HUD.UIUpdate` (`/Game/Framework/BP_player.WB_Hud_ref` _asbp_player) (`KismetTextLibrary.Conv_IntToText` (`self.Orbs`))))